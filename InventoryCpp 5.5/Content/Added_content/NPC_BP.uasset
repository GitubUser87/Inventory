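; NPC Blueprint that opens an inventory screen when the player walks into its trigger box, as part of an item request interaction.
; On overlap begin with the player character it creates an Inventory_BP widget, adds it to the viewport and switches to game-and-UI input with the mouse cursor shown.
; On overlap end it removes the widget and restores game-only input with the cursor hidden.
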(event OnComponentBeginOverlap(Box)
  (params (OverlappedComponent :type Primitive%20Component%20Object%20Reference) (OtherActor :type Actor%20Object%20Reference) (OtherComp :type Primitive%20Component%20Object%20Reference) (OtherBodyIndex :type Integer) (bFromSweep :type Boolean) (SweepResult :type Hit%20Result%20Structure%20%28by%20ref%29))
  (bind _returnvalue (Game|GetPlayerController 0))
  ;[1 1 1] Ask for item
  (if (== OtherActor (Game|GetPlayerCharacter 0))
    (bind _returnvalue_2 (UserInterface|CreateWidget "/Game/Added_content/Inventory_BP.Inventory_BP_C"))
    (UserInterface|Viewport|AddtoViewport _returnvalue_2 0)
    (Input|SetInputModeGameandUI _returnvalue _returnvalue_2 "DoNotLock" true false)
    (Variables|/Script/Engine.PlayerController|SetbShowMouseCursor _returnvalue true)))

(event OnComponentEndOverlap(Box)
  (params (OverlappedComponent :type Primitive%20Component%20Object%20Reference) (OtherActor :type Actor%20Object%20Reference) (OtherComp :type Primitive%20Component%20Object%20Reference) (OtherBodyIndex :type Integer))
  (bind _returnvalue (Game|GetPlayerController 0))
  ;[1 1 1] Ask for item
  (if (== OtherActor (Game|GetPlayerCharacter 0))
    (Widget|RemovefromParent (stale OnComponentBeginOverlap(Box) _returnvalue_2))
    (Input|SetInputModeGameOnly _returnvalue false)
    (Variables|/Script/Engine.PlayerController|SetbShowMouseCursor _returnvalue false)))

(fn ConstructionScript)